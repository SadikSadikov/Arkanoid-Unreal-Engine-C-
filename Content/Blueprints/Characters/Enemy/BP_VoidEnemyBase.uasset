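; Base Blueprint for a Void enemy that moves at constant speed, climbing obstacles and falling when unsupported.
; Tick applies Direction as a swept offset; blocking hits steer it using forward vector dot impact normal.
; Walls send it upward, ceilings downward, and floor hits alternate it between -X and +X.
; A looping downward box trace forces descent and sets Block, suspending steering until ground is detected again.
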(event Custom|CheckForGorund
  (bind _returnvalue (Transformation|GetActorLocation))
  (bind (_x _y _z) (Math|Vector|BreakVector _returnvalue))
  (bind _outhit (Collision|BoxTraceByChannel _returnvalue (Math|Vector|MakeVector _x _y (- _z 1.5e+02)) "40.000000,50.000000,40.000000" "0, 0, 0" "TraceTypeQuery1" false 0 "ForOneFrame" true "(R=1.000000,G=0.000000,B=0.000000,A=1.000000)" "(R=0.000000,G=1.000000,B=0.000000,A=1.000000)" 0.2))
  (if (.bBlockingHit (Collision|BreakHitResult _outhit))
    (Variables|Default|SetbBlock false)
    (else
      (Variables|Default|SetbBlock true)
      (Variables|Default|SetDirection (Math|Vector|MakeVector 0.0 0.0 -1.0)))))

(event EventBeginPlay
  (Utilities|Time|SetTimerbyEvent (delegate Custom|CheckForGorund) 0.2 true))

(event Collision|EventActorBeginOverlap
  (params (OtherActor :type Actor%20Object%20Reference)))

(event EventTick
  (params (DeltaSeconds :type Float%20%28single-precision%29))
  (Variables|Default|SetVelocity (* (Math|Vector|Normalize (Variables|Default|GetDirection)) 2e+02 DeltaSeconds))
  (bind _sweephitresult (Transformation|AddActorWorldOffset (Variables|Default|GetVelocity) true))
  (if (not (Variables|Default|GetbBlock))
    (if (.bBlockingHit (Collision|BreakHitResult _sweephitresult))
      (if (== (Math|Vector|DotProduct (Transformation|GetActorForwardVector) (.ImpactNormal (Collision|BreakHitResult _sweephitresult))) 0.0)
        (if (> (.Z (Math|Vector|BreakVector (Variables|Default|GetDirection))) 0.0)
          (Variables|Default|SetDirection "0.000000,0.000000,-1.000000")
          (elif (>= (Variables|Default|GetLastleftRightDirection) 0.0)
            (bind _output_get (Variables|Default|SetDirection "-1.000000,0.000000,0.000000"))
            (Variables|Default|SetLastleftRightDirection (.X (Math|Vector|BreakVector _output_get)))
            (else
              (bind _output_get_2 (Variables|Default|SetDirection "1.000000,0.000000,0.000000"))
              (Variables|Default|SetLastleftRightDirection (.X (Math|Vector|BreakVector _output_get_2))))))
        (elif (> (Math|Vector|DotProduct (Transformation|GetActorForwardVector) (.ImpactNormal (Collision|BreakHitResult _sweephitresult))) 0.0)
          (Variables|Default|SetDirection "0.000000,0.000000,1.000000")
          (else
            (Variables|Default|SetDirection "0.000000,0.000000,1.000000")))))))

(fn ConstructionScript)